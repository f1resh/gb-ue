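; Test Blueprint that extrudes a polygon on a static mesh actor clicked with the mouse, using runtime mesh editing.
; It shows the cursor on BeginPlay, then on left mouse release traces from the cursor into the world.
; A StaticMeshActor hit becomes an EditableMesh, whose polygon at PoligonIndex is extruded by a fixed negative distance and committed.
; The index comes from a variable, not the hit result, and is printed afterward.
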(event `self.ReceiveBeginPlay`
  (set `self.bShowMouseCursor` true))

(event `Key|LeftMouseButton`
  (params (Key :type "Key Structure"))
  (bind (_worldlocation _worlddirection) (`self.DeprojectMousePositionToWorld`))
  (bind _poligonindex (`self.poligonIndex`))
  (:`Released`
    (bind (_outhit _returnvalue) (`KismetSystemLibrary.LineTraceSingle` :`Start` _worldlocation :`End` (+ _worldlocation (* _worlddirection 100000.0)) :`TraceChannel` "TraceTypeQuery1" :`DrawDebugType` "ForDuration"))
    (if _returnvalue
      (bind _asstatic_mesh_actor (cast `StaticMeshActor` (`.HitActor` (`GameplayStatics.BreakHitResult` _outhit))))
      (bind _returnvalue_2 (`EditableMeshFactory.MakeEditableMesh` (`StaticMeshActor.StaticMeshComponent` _asstatic_mesh_actor)))
      (`EditableMesh.StartModification` _returnvalue_2 "FirstInterim" "NoTopologyChange")
      (`EditableMesh.ExtrudePolygons` _returnvalue_2 (`|MakeArray` (`EditableMesh.MakePolygonID` _poligonindex)) -300.0 true)
      (`EditableMesh.EndModification` _returnvalue_2 false)
      (`EditableMesh.Commit` _returnvalue_2)
      (`KismetSystemLibrary.PrintString` (`KismetStringLibrary.Conv_IntToString` _poligonindex) true true (struct :`R` 0.98018 :`G` 1.0 :`A` 1.0) 5.0))))

(fn `UserConstructionScript`)